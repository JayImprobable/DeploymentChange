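; Player character Blueprint that serves as a keyboard trigger for client travel through the player controller.
; On BeginPlay it casts player controller 0 to MyPlayerController and caches it, printing a debug string for success or failure.
; Pressing J calls FirstClientTravel on the cached controller, with no validity check.
; Overlap, Tick and the construction script do nothing, and two IsServer checks are left unconnected.
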(event `self.ReceiveBeginPlay`
  (bind _asmy_player_controller (cast `MyPlayerController` (`GameplayStatics.GetPlayerController` 0))
    (:`then`
      (set `self.MyPlayerController` _asmy_player_controller)
      (`KismetSystemLibrary.PrintString` "???"))
    (:`CastFailed`
      (`KismetSystemLibrary.PrintString` "!!!"))))

(event `Key|J`
  (params (Key :type "Key Structure"))
  (:`Pressed`
    (`MyPlayerController.FirstClientTravel` (`self.MyPlayerController`))))

(fn `UserConstructionScript`)